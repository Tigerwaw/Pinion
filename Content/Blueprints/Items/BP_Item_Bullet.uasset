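; Ammo pickup item that refills the interacting player's bullets.
; Interact calls the parent behavior, then Use, which adds the item's ammo amount to the count stored on the player's inventory widget, capped at that widget's maximum.
; The capped branch prints the new count for debugging, and GetPromptType returns an empty string.
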(event `/Game/Blueprints/Interactables/Interact.Interact`
  (params (Player :type "/Game/CustomCharacter/PlayerCharacter/BP_ThirdPersonCharacter Object Reference"))
  (`parent.Interact` Player)
  (`/Game/Blueprints/Items/Use.Use` Player))

(event `/Game/Blueprints/Items/Use.Use`
  (params (Player :type "/Game/CustomCharacter/PlayerCharacter/BP_ThirdPersonCharacter Object Reference"))
  (bind _inventorywidget (`/Game/CustomCharacter/PlayerCharacter/BP_ThirdPersonCharacter.InventoryWidget` Player))
  (bind _maxammoamount (`/Game/Blueprints/UI/Inventory/Inventory.MaxAmmoAmount` _inventorywidget))
  (bind _returnvalue (+ (`/Game/Blueprints/UI/Inventory/Inventory.CurrentAmmoAmount` _inventorywidget) (`self.AmmoAmount`)))
  (if (> _returnvalue _maxammoamount)
    (bind _output_get (set `/Game/Blueprints/UI/Inventory/Inventory.CurrentAmmoAmount` _maxammoamount _inventorywidget))
    (`KismetSystemLibrary.PrintString` (`KismetStringLibrary.Conv_IntToString` _output_get))
    (else
      (bind _output_get_2 (set `/Game/Blueprints/UI/Inventory/Inventory.CurrentAmmoAmount` _returnvalue _inventorywidget)))))

(fn `GetPromptType`
  (returns (PromptType :type String))
  (return ""))

(fn `UserConstructionScript`
  (`parent.UserConstructionScript`))