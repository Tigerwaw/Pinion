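; Base Blueprint for items that the player can pick up, drop and use, showing a "pick up" prompt type.
; Interact passes the item info and the actor itself to the player's inventory widget and turns off the mesh's custom depth rendering.
; DropItem moves that same actor to the drop location and turns custom depth back on.
; Use only prints the item's name as a placeholder.
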(event `/Game/Blueprints/Interactables/Interact.Interact`
  (params (Player :type "/Game/CustomCharacter/PlayerCharacter/BP_ThirdPersonCharacter Object Reference"))
  ;[1 1 1] Pick up item (Interact)
  (`/Game/Blueprints/UI/Inventory/Inventory.AddToInventory` (`/Game/CustomCharacter/PlayerCharacter/BP_ThirdPersonCharacter.InventoryWidget` Player) (`self.ItemInfo`) self)
  (`PrimitiveComponent.SetRenderCustomDepth` (`self.ItemMesh`) false))

(event `DropItem`
  (params (DropLocation :type "Vector Structure"))
  ;[1 1 1] Drop Item
  (`SceneComponent.K2_SetWorldLocation` (`self.DefaultSceneRoot`) DropLocation false false)
  (`PrimitiveComponent.SetRenderCustomDepth` (`self.ItemMesh`) true))

(event `/Game/Blueprints/Items/Use.Use`
  (params (Player :type "/Game/CustomCharacter/PlayerCharacter/BP_ThirdPersonCharacter Object Reference"))
  (bind (_iteminfo_icon _iteminfo_name) (break `/Game/Blueprints/Items/ItemInfoStructure` (`self.ItemInfo`)))
  ;[1 1 1] Use
  (`KismetSystemLibrary.PrintString` (`KismetStringLibrary.Concat_StrStr` "Used item " _iteminfo_name)))

(fn `GetPromptType`
  (returns (PromptType :type String))
  (return "pick up"))

(fn `UserConstructionScript`)