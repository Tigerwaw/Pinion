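; BP_AI_Monster is an AI monster pawn with melee paw attacks, damage and death reactions, and sounds.
; On BeginPlay it hands its behavior tree and AnimBP to AIC_Monster, then notifies that controller of damage, death and fear.
; Attack plays a montage, while a toggleable paw hitbox, initially off, deals random ranged damage to overlapped actors.
; Capsule overlaps with components tagged FearComponent send the fear source location to the controller.
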(event `self.ReceiveBeginPlay`
  ;[1 1 1] Initialize Variables
  (bind _asanim_bp_monster (cast `/Game/CustomCharacter/Monster/Animations/AnimBP_Monster` (`SkeletalMeshComponent.GetAnimInstance` (`self.Mesh`))))
  (set `self.As Anim BP Monster` _asanim_bp_monster)
  (bind _asaic_monster (cast `/Game/Blueprints/AI/AIC_Monster` (`AIBlueprintHelperLibrary.GetAIController` self)))
  (bind _output_get (set `self.AI_Controller` _asaic_monster))
  (`/Game/Blueprints/AI/AIC_Monster.Setup AIC` _output_get (`self.BT`) (`self.As Anim BP Monster`))
  (`self.ToggleHitbox` "NoCollision"))

(event `/Game/Blueprints/CharacterStats/Health.Take Damage`
  (params (DamageAmount :type "Float (double-precision)") (HitLocation :type "Vector Structure") (DamagedBy :type "Actor Object Reference"))
  (`parent.Take Damage` DamageAmount HitLocation DamagedBy)
  (`/Game/Blueprints/AI/AIC_Monster.Pawn_Damaged` (`self.AI_Controller`))
  (`GameplayStatics.PlaySoundAtLocation` (`self.HurtSound`) (`self.K2_GetActorLocation`) (struct) 1.0 1.0 0.0 null null null null))

(event `/Game/Blueprints/CharacterStats/Health.Death`
  (`parent.Death`)
  (`/Game/Blueprints/AI/AIC_Monster.Pawn_Death` (`self.AI_Controller`))
  (`GameplayStatics.PlaySoundAtLocation` (`self.DeathSound`) (`self.K2_GetActorLocation`) (struct) 1.0 1.0 0.0 null null null null))

(event `Attack`
  ;[1 1 1] Attack
  (`|PlayMontage` (`self.Mesh`) (`self.AttackAnimation`)
    (:`then`
      (`GameplayStatics.PlaySoundAtLocation` (`self.AttackSound`) (`self.K2_GetActorLocation`) (struct) 1.0 1.0 0.0 null null null null))))

(event `self.PawHitbox.OnComponentBeginOverlap`
  (params (OverlappedComponent :type "PrimitiveComponent Object Reference") (OtherActor :type "Actor Object Reference") (OtherComp :type "PrimitiveComponent Object Reference") (OtherBodyIndex :type Integer) (bFromSweep :type Boolean) (SweepResult :type "HitResult Structure (by ref)"))
  (bind _returnvalue (`self.K2_GetActorLocation` OtherActor))
  (bind _damage (`self.Damage`))
  ;[1 1 1] Paw Hitbox Overlap
  (if (!= OtherActor self)
    (message `/Game/Blueprints/CharacterStats/Health.Take Damage` OtherActor (`KismetMathLibrary.RandomFloatInRange` (`.Value` (break `FloatRangeBound` (break `FloatRange` _damage))) (`.Value` (break `FloatRangeBound` (`.UpperBound` (break `FloatRange` _damage))))) _returnvalue self)
    (`GameplayStatics.PlaySoundAtLocation` (`self.AttackHitSound`) _returnvalue (struct) 1.0 1.0 0.0 null null null null)))

(event `ToggleHitbox`
  (params (NewType :type "ECollisionEnabled Enum" :default "NoCollision"))
  ;[1 1 1] Toggle Hitbox
  (`PrimitiveComponent.SetCollisionEnabled` (`self.PawHitbox`) NewType))

(event `self.CapsuleComponent.OnComponentBeginOverlap`
  (params (OverlappedComponent :type "PrimitiveComponent Object Reference") (OtherActor :type "Actor Object Reference") (OtherComp :type "PrimitiveComponent Object Reference") (OtherBodyIndex :type Integer) (bFromSweep :type Boolean) (SweepResult :type "HitResult Structure (by ref)"))
  ;[1 1 1] On Hitbox Collision
  (if (`ActorComponent.ComponentHasTag` OtherComp "FearComponent")
    (`/Game/Blueprints/AI/AIC_Monster.Pawn_Fear` (`self.AI_Controller`) (`SceneComponent.K2_GetComponentLocation` OtherComp))))

(fn `UserConstructionScript`)