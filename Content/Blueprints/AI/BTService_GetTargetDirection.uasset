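; Behavior tree service that predicts where the AI's Target is heading and writes that point to the GoalLocation blackboard key.
; Each tick it takes the normalized direction from TargetsLastPosition to the target's current location and projects PredictionDistance ahead of the target.
; It then stores the current location as TargetsLastPosition for the next tick, so the lead is a fixed distance regardless of target speed.
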(event `self.ReceiveTickAI`
  (params (OwnerController :type "AIController Object Reference") (ControlledPawn :type "Pawn Object Reference") (DeltaSeconds :type "Float (single-precision)"))
  (bind _returnvalue (`Actor.K2_GetActorLocation` (`BTFunctionLibrary.GetBlackboardValueAsActor` (`self.Target`))))
  (`BTFunctionLibrary.SetBlackboardValueAsVector` (`self.GoalLocation`) (+ _returnvalue (* (`KismetMathLibrary.Normal` (- _returnvalue (`BTFunctionLibrary.GetBlackboardValueAsVector` (`self.TargetsLastPosition`)))) (`self.PredictionDistance`))))
  (`BTFunctionLibrary.SetBlackboardValueAsVector` (`self.TargetsLastPosition`) _returnvalue))