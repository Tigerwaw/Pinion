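; Behavior tree task that sets the AI controller's focus on the blackboard Target only when it has line of sight to it.
; It traces on the Camera channel from the pawn to Target, read as a vector, ignoring the pawn itself.
; If the hit actor matches Target read as an actor, it becomes the focus; otherwise focus is cleared.
; The task always finishes successfully.
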(event `self.ReceiveExecuteAI`
  (params (OwnerController :type "AIController Object Reference") (ControlledPawn :type "Pawn Object Reference"))
  (bind _aicontroller (`self.AIController`))
  (set `self.AIController` OwnerController)
  (bind _outhit (`KismetSystemLibrary.LineTraceSingle` (`Actor.K2_GetActorLocation` ControlledPawn) (`BTFunctionLibrary.GetBlackboardValueAsVector` (`self.Target`)) "TraceTypeQuery2" false (`|MakeArray` ControlledPawn :!type "Actor Object Reference")))
  (if (== (`.HitActor` (`GameplayStatics.BreakHitResult` _outhit)) (`BTFunctionLibrary.GetBlackboardValueAsActor` (`self.Target`)))
    (`AIController.K2_SetFocus` _aicontroller (`.HitActor` (`GameplayStatics.BreakHitResult` _outhit)))
    (else
      (`AIController.K2_ClearFocus` _aicontroller)))
  (`self.FinishExecute` true))