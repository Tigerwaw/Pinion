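; Test AI pawn that runs a behavior tree and can be damaged and killed.
; On BeginPlay it passes its behavior tree and the first player's pawn, as the sense target, to its AIC_Test controller.
; TakeDamage subtracts from Health in the Stats struct, spawning a blood burst at the hit location while health remains, or calling Death, which destroys the actor.
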(event `self.ReceiveBeginPlay`
  ;[1 1 1] Initialize Variables
  (bind _asaic_test (cast `/Game/Blueprints/AI/AIC_Test` (`AIBlueprintHelperLibrary.GetAIController` self)))
  (`/Game/Blueprints/AI/AIC_Test.Setup AIC` _asaic_test (`self.BT`) (`GameplayStatics.GetPlayerPawn` 0)))

(event `self.Take Damage`
  (params (DamageAmount :type "Float (double-precision)") (HitLocation :type "Vector Structure"))
  (bind (_stats_health _stats_maxhealth) (break `/Game/Blueprints/CharacterStats/CharacterStats` (`self.Stats`)))
  ;[1 1 1] Take Damage
  (bind _output_get (set `self.Stats` (make `/Game/Blueprints/CharacterStats/CharacterStats` (- _stats_health DamageAmount) _stats_maxhealth)))
  (if (<= (break `/Game/Blueprints/CharacterStats/CharacterStats` _output_get) 0.0)
    (`self.Death`)
    (else
      (`NiagaraFunctionLibrary.SpawnSystemAtLocation` "/Game/Particles/PS_Blood_Burst.PS_Blood_Burst" HitLocation))))

(event `self.Death`
  ;[1 1 1] Death
  (`self.K2_DestroyActor`))

(fn `UserConstructionScript`)