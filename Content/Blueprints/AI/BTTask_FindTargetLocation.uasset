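; Behavior tree task that picks a random navigable location around the Target actor and writes it to the TargetLocation blackboard key.
; It offsets DistanceFromPlayer from the target along a random cone aimed at the pawn, whose 180-degree half-angle allows any 3D direction.
; A small-radius navmesh query around that point supplies the location, and the task always finishes successfully without checking the query result.
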(event `self.ReceiveExecuteAI`
  (params (OwnerController :type "AIController Object Reference") (ControlledPawn :type "Pawn Object Reference"))
  (bind _returnvalue (`Actor.K2_GetActorLocation` (`BTFunctionLibrary.GetBlackboardValueAsActor` (`self.Target`))))
  (`BTFunctionLibrary.SetBlackboardValueAsVector` (`self.TargetLocation`) (`NavigationSystemV1.K2_GetRandomLocationInNavigableRadius` (+ _returnvalue (* (`KismetMathLibrary.RandomUnitVectorInConeInDegrees` (`KismetMathLibrary.GetDirectionUnitVector` _returnvalue (`Actor.K2_GetActorLocation` ControlledPawn)) 180.0) (`self.DistanceFromPlayer`))) 50.0 null null))
  (`self.FinishExecute` true))