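; Blueprint function library of AI helpers for writing Blackboard values from an AI controller.
; Separate functions set Bool, Object, Vector and Enum entries by key name.
; Each gets the controller's Blackboard and calls the matching typed setter, converting the key with MakeLiteralName, with no validity check on the Blackboard.
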(fn `SetBB_Bool`
  (params (`AI Controller` :type "AIController Object Reference") (KeyName :type Name) (Bool :type Boolean))
  (`BlackboardComponent.SetValueAsBool` (`AIBlueprintHelperLibrary.GetBlackboard` `AI Controller`) (`KismetSystemLibrary.MakeLiteralName` KeyName) Bool))

(fn `SetBB_Enum`
  (params (`AI Controller` :type "Actor Object Reference") (KeyName :type Name) (EnumValue :type "/Game/Blueprints/AI/AI_ActionStates Enum" :default "NewEnumerator0"))
  (`BlackboardComponent.SetValueAsEnum` (`AIBlueprintHelperLibrary.GetBlackboard` `AI Controller`) (`KismetSystemLibrary.MakeLiteralName` KeyName) EnumValue))

(fn `SetBB_Object`
  (params (`AI Controller` :type "Actor Object Reference") (KeyName :type Name) (Object :type "Object Object Reference"))
  (`BlackboardComponent.SetValueAsObject` (`AIBlueprintHelperLibrary.GetBlackboard` `AI Controller`) (`KismetSystemLibrary.MakeLiteralName` KeyName) Object))

(fn `SetBB_Vector`
  (params (`AI Controller` :type "Actor Object Reference") (KeyName :type Name) (Vector :type "Vector Structure"))
  (`BlackboardComponent.SetValueAsVector` (`AIBlueprintHelperLibrary.GetBlackboard` `AI Controller`) (`KismetSystemLibrary.MakeLiteralName` KeyName) Vector))