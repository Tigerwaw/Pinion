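; AIC_Test is an AI controller that runs a supplied behavior tree and tracks one designated target pawn through PawnSensing.
; Its setup event stores the tree and target, then writes the target and the controlled pawn's starting location to the blackboard.
; Sightings of that target flag it as visible and recently seen and record its position.
; A retriggerable delay of twice the sensing interval clears only the visibility flag once sightings stop.
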(event `Setup AIC`
  (params (BT :type "BehaviorTree Object Reference") (PawnSenseTarget :type "Pawn Object Reference"))
  (set `self.BT` BT)
  (set `self.PawnSenseTarget` PawnSenseTarget)
  (`self.RunBehaviorTree` (`self.BT`))
  (`/Game/Blueprints/AI/FuncLib_AI.SetBB_Object` self "Target" (`self.PawnSenseTarget`))
  (`/Game/Blueprints/AI/FuncLib_AI.SetBB_Vector` self "Origin" (`self.K2_GetActorLocation` (`self.K2_GetPawn`))))

(event `self.PawnSensing.OnSeePawn`
  (params (Pawn :type "Pawn Object Reference"))
  (if (== Pawn (`self.PawnSenseTarget`))
    (`|ExecutionSequence`
      (:`then_0`
        (`/Game/Blueprints/AI/FuncLib_AI.SetBB_Bool` self "CanSeeTarget" true)
        (`KismetSystemLibrary.RetriggerableDelay` (* (`PawnSensingComponent.SensingInterval` (`self.PawnSensing`)) 2.0))
        (`/Game/Blueprints/AI/FuncLib_AI.SetBB_Bool` self "CanSeeTarget"))
      (:`then_1`
        (`/Game/Blueprints/AI/FuncLib_AI.SetBB_Bool` self "RecentlySeenTarget" true))
      (:`then_2`
        (`/Game/Blueprints/AI/FuncLib_AI.SetBB_Vector` self "PlayersLastSeenPosition" (`self.K2_GetActorLocation` (`self.PawnSenseTarget`)))))))

(fn `UserConstructionScript`)