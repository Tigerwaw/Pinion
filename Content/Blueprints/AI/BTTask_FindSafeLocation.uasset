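; Behavior tree task that picks a flee location for an AI pawn away from a blackboard fear source.
; It takes a random direction in a cone around the source-to-pawn vector and scales it by DistanceToBack.
; That vector, not offset by the pawn's location, seeds a small-radius random navigable point search.
; The result is written to SafeLocationKey, and the task always finishes successfully.
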(event `self.ReceiveExecuteAI`
  (params (OwnerController :type "AIController Object Reference") (ControlledPawn :type "Pawn Object Reference"))
  (`BTFunctionLibrary.SetBlackboardValueAsVector` (`self.SafeLocationKey`) (`NavigationSystemV1.K2_GetRandomLocationInNavigableRadius` (* (`KismetMathLibrary.RandomUnitVectorInConeInDegrees` (`KismetMathLibrary.GetDirectionUnitVector` (`BTFunctionLibrary.GetBlackboardValueAsVector` (`self.FearSource`)) (`Actor.K2_GetActorLocation` ControlledPawn)) 60.0) (`self.DistanceToBack`)) 50.0 null null))
  (`self.FinishExecute` true))