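; DamageArea is a hazard volume that repeatedly damages the third-person character while it overlaps the HurtBox.
; On overlap begin it stores the character and starts a looping timer at DamageInterval, so the first hit lands after one interval.
; Each tick casts the stored Player to Health and calls TakeDamage with DamageAmount and a zero hit location.
; Overlap end by that character class clears the single timer handle.
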(event `DealDamage`
  (bind _ashealth (cast `/Game/Blueprints/CharacterStats/Health` (`self.Player`)))
  (`/Game/CustomCharacter/PlayerCharacter/BP_ThirdPersonCharacter.Take Damage` _ashealth (`self.DamageAmount`) (0.0 0.0 0.0)))

(event `self.HurtBox.OnComponentBeginOverlap`
  (params (OverlappedComponent :type "PrimitiveComponent Object Reference") (OtherActor :type "Actor Object Reference") (OtherComp :type "PrimitiveComponent Object Reference") (OtherBodyIndex :type Integer) (bFromSweep :type Boolean) (SweepResult :type "HitResult Structure (by ref)"))
  (bind _asbp_third_person_character (cast `/Game/CustomCharacter/PlayerCharacter/BP_ThirdPersonCharacter` OtherActor))
  (set `self.Player` _asbp_third_person_character)
  (bind _returnvalue (`KismetSystemLibrary.K2_SetTimerDelegate` (delegate `DealDamage`) (`self.DamageInterval`) true))
  (set `self.Timer` _returnvalue))

(event `self.HurtBox.OnComponentEndOverlap`
  (params (OverlappedComponent :type "PrimitiveComponent Object Reference") (OtherActor :type "Actor Object Reference") (OtherComp :type "PrimitiveComponent Object Reference") (OtherBodyIndex :type Integer))
  (cast `/Game/CustomCharacter/PlayerCharacter/BP_ThirdPersonCharacter` OtherActor)
  (`KismetSystemLibrary.K2_ClearAndInvalidateTimerHandle` (`self.Timer`)))

(fn `UserConstructionScript`)