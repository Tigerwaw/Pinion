(fn `Create Sound`
  (params (Instigator :type "Pawn Object Reference") (Sound :type "SoundBase Object Reference") (Location :type "Vector Structure") (MakeNoiseEvent :type Boolean))
  (locals (_PawnNoiseEmitter :type "PawnNoiseEmitterComponent Object Reference") (_Instigator :type "Pawn Object Reference") (_Sound :type "SoundBase Object Reference") (_Location :type "Vector Structure") (_MakeNoiseEvent :type Boolean))
  (bind __instigator (`local._Instigator`))
  (set `local._Instigator` Instigator)
  (set `local._Sound` Sound)
  (set `local._Location` Location)
  (set `local._MakeNoiseEvent` MakeNoiseEvent)
  (`GameplayStatics.PlaySoundAtLocation` (`local._Instigator`) (`local._Sound`) (`local._Location`) (struct) 1.0 1.0 0.0 null null null null)
  (if (`local._MakeNoiseEvent`)
    (`Pawn.PawnMakeNoise` __instigator 1.0 (`local._Location`) false __instigator)))

(fn `GetTimeDifference`
  (params (Caller :type "Object Object Reference") (StartTime :type "Float (double-precision)") (Duration :type "Float (double-precision)"))
  (returns (IsDone :type Boolean))
  (return (>= (`KismetSystemLibrary.GetGameTimeInSeconds` Caller) (+ StartTime Duration))))