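; Double-door interactable that toggles between open and closed through the OpenCloseDoor event.
; Separate right and left timelines yaw each leaf, playing forward to open and in reverse to close.
; Knob and squeak sounds play as movement starts; both timelines' Finished outputs share the closing-sound check.
; BeginPlay sets only Door1's starting yaw from IsOpen, leaving the other leaf untouched.
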(event `self.ReceiveBeginPlay`
  (`parent.ReceiveBeginPlay`)
  (if (`self.IsOpen`)
    (`SceneComponent.K2_SetRelativeRotation` (`self.Door1`) (struct :`Yaw` 270.0) false false)
    (else
      (`SceneComponent.K2_SetRelativeRotation` (`self.Door1`) (struct :`Yaw` 180.0) false false))))

(event `self.OpenCloseDoor`
  (bind _output_get (set `self.IsOpen` (not (`self.IsOpen`))))
  (if _output_get
    (`|ExecutionSequence`
      (:`then_0`
        (`self.MakeSound` (`self.DoorknobAudio`))
        (`self.MakeSound` (`self.DoorSqueakAudio`))
        (bind (_direction _door_open_track) (`Timeline|RightDoor_Timeline` :!label _label)
          (:`Update`
            (`SceneComponent.K2_SetRelativeRotation` (`self.Door`) (`KismetMathLibrary.MakeRotator` 0.0 0.0 _door_open_track) false false))
          (:`Finished`
            (if (not (`self.IsOpen`)) :!label _label_2
              (`self.MakeSound` (`self.DoorClosingAudio`))))))
      (:`then_1`
        (bind (_direction_2 _door_open_track_2) (`Timeline|LeftDoor_Timeline` :!label _label_3)
          (:`Update`
            (`SceneComponent.K2_SetRelativeRotation` (`self.Door1`) (`KismetMathLibrary.MakeRotator` 0.0 0.0 _door_open_track_2) false false))
          (:`Finished`
            (goto _label_2)))))
    (else
      (`|ExecutionSequence`
        (:`then_0`
          (`self.MakeSound` (`self.DoorSqueakAudio`))
          (goto _label :!via `Reverse`))
        (:`then_1`
          (goto _label_3 :!via `Reverse`))))))

(fn `GetPromptType`
  (returns (PromptType :type String))
  (bind _prompttype (`parent.GetPromptType`))
  (return _prompttype))

(fn `UserConstructionScript`
  (`parent.UserConstructionScript`))