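; Interactable ladder that the player toggles on and off to climb, shown with a "to climb" prompt.
; Getting on switches the interactor to Flying movement, disables orient-to-movement and snaps it in front of the ladder, facing it; getting off restores both settings.
; Leaving the trigger box while climbing dismounts and nudges the character to the ladder's opposite side.
; The construction script stacks mesh segments by Height and resizes the box to match.
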(event `/Game/Blueprints/Interactables/Interact.Interact`
  (params (Player :type "/Game/CustomCharacter/PlayerCharacter/BP_ThirdPersonCharacter Object Reference"))
  (`parent.Interact` Player)
  (`self.ToggleClimbingLadder`))

(event `ToggleClimbingLadder`
  (if (`/Game/CustomCharacter/PlayerCharacter/BP_ThirdPersonCharacter.IsOnLadder` (`self.Interactor`))
    (`self.GetOffLadder`)
    (else
      (`self.GetOnLadder`))))

(event `GetOnLadder`
  (bind _interactor (`self.Interactor`))
  (bind _defaultsceneroot (`self.DefaultSceneRoot`))
  (bind (_returnvalue_roll _returnvalue_pitch) (`KismetMathLibrary.BreakRotator` (`self.K2_GetActorRotation` (`self.Interactor`))))
  (bind (_returnvalue_roll_2 _returnvalue_pitch_2 _returnvalue_yaw) (`KismetMathLibrary.BreakRotator` (`SceneComponent.K2_GetComponentRotation` (`self.DefaultSceneRoot`))))
  (bind (_returnvalue_x _returnvalue_y _returnvalue_z) (`KismetMathLibrary.BreakVector` (`self.K2_GetActorLocation` (`self.Interactor`))))
  (bind (_returnvalue_x_2 _returnvalue_y_2) (`KismetMathLibrary.BreakVector` (`SceneComponent.K2_GetComponentLocation` _defaultsceneroot)))
  (bind _charactermovement (`Character.CharacterMovement` _interactor))
  (set `/Game/CustomCharacter/PlayerCharacter/BP_ThirdPersonCharacter.IsOnLadder` true _interactor)
  (`CharacterMovementComponent.SetMovementMode` _charactermovement "MOVE_Flying" 0)
  (set `CharacterMovementComponent.bOrientRotationToMovement` false _charactermovement)
  (`self.K2_SetActorLocationAndRotation` (`self.Interactor`) (+ (* (`SceneComponent.GetForwardVector` _defaultsceneroot) 50.0) (`KismetMathLibrary.MakeVector` _returnvalue_x_2 _returnvalue_y_2 _returnvalue_z)) (`KismetMathLibrary.MakeRotator` _returnvalue_roll _returnvalue_pitch (- _returnvalue_yaw 180.0)) false false))

(event `GetOffLadder`
  (bind _interactor (`self.Interactor`))
  (bind _charactermovement (`Character.CharacterMovement` _interactor))
  (set `/Game/CustomCharacter/PlayerCharacter/BP_ThirdPersonCharacter.IsOnLadder` false _interactor)
  (`CharacterMovementComponent.SetMovementMode` _charactermovement "MOVE_Walking" 0)
  (set `CharacterMovementComponent.bOrientRotationToMovement` true _charactermovement))

(event `self.Box.OnComponentEndOverlap`
  (params (OverlappedComponent :type "PrimitiveComponent Object Reference") (OtherActor :type "Actor Object Reference") (OtherComp :type "PrimitiveComponent Object Reference") (OtherBodyIndex :type Integer))
  (bind _defaultsceneroot (`self.DefaultSceneRoot`))
  (bind (_returnvalue_x _returnvalue_y _returnvalue_z) (`KismetMathLibrary.BreakVector` (`self.K2_GetActorLocation` (`self.Interactor`))))
  (bind (_returnvalue_x_2 _returnvalue_y_2) (`KismetMathLibrary.BreakVector` (`SceneComponent.K2_GetComponentLocation` _defaultsceneroot)))
  (if (`/Game/CustomCharacter/PlayerCharacter/BP_ThirdPersonCharacter.IsOnLadder` (`self.Interactor`))
    (`self.GetOffLadder`)
    (`self.K2_SetActorLocation` (`self.Interactor`) (+ (* (`KismetMathLibrary.NegateVector` (`SceneComponent.GetForwardVector` _defaultsceneroot)) 50.0) (`KismetMathLibrary.MakeVector` _returnvalue_x_2 _returnvalue_y_2 _returnvalue_z)) false false)))

(fn `GetPromptType`
  (returns (PromptType :type String))
  (return "to climb"))

(fn `UserConstructionScript`
  (bind _returnvalue (+ (`self.Height`) 1))
  (`parent.UserConstructionScript`)
  (for _index (range (+ (`self.Height`) 1))
    (`AddComponent|NODE_AddStaticMeshComponent-0` :`RelativeTransform` (`KismetMathLibrary.MakeTransform` (`KismetMathLibrary.MakeVector` 0.0 -40.0 (* _index 150.0)) (struct :`Pitch` 90.0 :`Yaw` 180.0 :`Roll` -90.0)))
    (`SceneComponent.K2_SetRelativeTransform` (`self.Box`) (`KismetMathLibrary.MakeTransform` (`KismetMathLibrary.MakeVector` 30.0 0.0 (* _returnvalue 75.0)) (struct) (`KismetMathLibrary.MakeVector` 1.0 2.0 (* _returnvalue 2.25))) false false)))