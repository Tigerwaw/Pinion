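; BP_Interactable_Base is a base interactable that gates success on items in the interacting player's inventory.
; On Interact it searches the player's inventory widget slots for each ItemsNeeded key by name, requiring a slot for every one.
; If all are found, it removes items whose map value flags consumption and fires InteractSuccess; otherwise it fires InteractFail.
; Both outcome events only print messages here, and GetPromptType returns an "Interact" prompt.
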(event `/Game/Blueprints/Interactables/Interact.Interact`
  (params (Player :type "/Game/CustomCharacter/PlayerCharacter/BP_ThirdPersonCharacter Object Reference"))
  (set `self.Interactor` Player)
  (`self.CheckForRequiredItems`))

(event `InteractSuccess`
  (`KismetSystemLibrary.PrintString` "Successfully Interacted"))

(event `InteractFail`
  (`KismetSystemLibrary.PrintString` "Failed to Interact"))

(fn `CheckForRequiredItems`
  (locals (SlotsOfFoundItems :type "Array of /Game/Blueprints/UI/Inventory/InventorySlot Object Reference"))
  (bind _keys (`BlueprintMapLibrary.Map_Keys` (`self.ItemsNeeded`)))
  (for _array_element _keys
    (for _array_element_2 (`/Game/Blueprints/UI/Inventory/Inventory.InventorySlotArray` (`/Game/CustomCharacter/PlayerCharacter/BP_ThirdPersonCharacter.InventoryWidget` (`self.Interactor`)))
      (bind (_item_info_icon _item_info_name) (break `/Game/Blueprints/Items/ItemInfoStructure` (`/Game/Blueprints/UI/Inventory/InventorySlot.Item Info` _array_element_2)))
      (if (`KismetStringLibrary.EqualEqual_StrStr` _array_element _item_info_name)
        (`KismetArrayLibrary.Array_AddUnique` (`local.SlotsOfFoundItems`) _array_element_2)
        (break))))
  (if (== (`BlueprintMapLibrary.Map_Length` (`self.ItemsNeeded`)) (`KismetArrayLibrary.Array_Length` (`local.SlotsOfFoundItems`)))
    (`self.ConsumeItems` (`local.SlotsOfFoundItems`))
    (`self.InteractSuccess`)
    (else
      (`self.InteractFail`))))

(fn `ConsumeItems`
  (params (ItemSlotsToConsume :type "Array of /Game/Blueprints/UI/Inventory/InventorySlot Object Reference"))
  (for _array_element ItemSlotsToConsume
    (bind _keys (`BlueprintMapLibrary.Map_Keys` (`self.ItemsNeeded`)))
    (for _array_element_2 _keys
      (bind (_item_info_icon _item_info_name) (break `/Game/Blueprints/Items/ItemInfoStructure` (`/Game/Blueprints/UI/Inventory/InventorySlot.Item Info` _array_element)))
      (if (and (`KismetStringLibrary.EqualEqual_StrStr` _array_element_2 _item_info_name) (`BlueprintMapLibrary.Map_Find` (`self.ItemsNeeded`) _array_element_2))
        (`/Game/Blueprints/UI/Inventory/InventorySlot.RemoveItem` _array_element)))))

(fn `GetPromptType`
  (returns (PromptType :type String))
  (return "Interact"))

(fn `UserConstructionScript`)