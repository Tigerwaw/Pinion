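; Interactable door that swings open and closed on a timeline-driven yaw rotation and can start locked.
; Locked doors defer to the inherited required-item check or, with no items needed, use a dot product so they unlock only from behind the actor's forward vector.
; A successful interaction toggles the door and clears the lock.
; The prompt type switches between open, close and unlock to match the current state.
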(event `/Game/Blueprints/Interactables/Interact.Interact`
  (params (Player :type "/Game/CustomCharacter/PlayerCharacter/BP_ThirdPersonCharacter Object Reference"))
  ;[1 1 1] Interact
  (`parent.Interact` Player)
  (if (`self.IsLocked`)
    (if (`BlueprintMapLibrary.Map_IsEmpty` (`self.ItemsNeeded`))
      (if (`self.Check Interact Direction`)
        (`self.InteractSuccess`)
        (else
          (`self.InteractFail`)))
      (else
        (`self.CheckForRequiredItems`)))
    (else
      (`self.InteractSuccess`))))

(event `self.InteractSuccess`
  (`parent.InteractSuccess`)
  (`self.OpenCloseDoor`)
  (set `self.IsLocked` false))

(event `self.InteractFail`
  (`parent.InteractFail`))

(event `OpenCloseDoor`
  ;[1 1 1] Open and Close Door
  (bind _output_get (set `self.IsOpen` (not (`self.IsOpen`))))
  (if _output_get
    (bind (_direction _door_open_track) (`Timeline|Door_Timeline` :!label _label)
      (:`Update`
        (`SceneComponent.K2_SetRelativeRotation` (`self.Door`) (`KismetMathLibrary.MakeRotator` 0.0 0.0 _door_open_track) false false)))
    (else
      (goto _label :!via `Reverse`))))

(fn `Check Interact Direction`
  (returns (IsInFrontOfDoor :type Boolean))
  (return (< (`KismetMathLibrary.Dot_VectorVector` (`self.GetActorForwardVector`) (`KismetMathLibrary.GetDirectionUnitVector` (`self.K2_GetActorLocation`) (`self.K2_GetActorLocation` (`self.Interactor`)))) 0.0)))

(fn `GetPromptType`
  (returns (PromptType :type String))
  (if (`self.IsOpen`)
    (return "close")
    (elif (`self.IsLocked`)
      (return "unlock")
      (else
        (return "open")))))

(fn `UserConstructionScript`)