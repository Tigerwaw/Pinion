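; Equippable torch whose light and fire particles show while equipped, and whose primary action swings it, enabling a fear collider during the montage.
; Each swing needs enough light, then drains the light level when the montage completes or is interrupted.
; Light level scales point light intensity and Niagara spawn rate, and a looping timer restores it to maximum, paused while swinging.
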(event `self.ReceiveBeginPlay`
  ;[1 1 1] Begin Play
  (`parent.ReceiveBeginPlay`)
  (`PrimitiveComponent.SetCollisionEnabled` (`self.FearCollider`) "NoCollision")
  (`SceneComponent.SetVisibility` (`self.PointLight`) false false)
  (`ActorComponent.SetActive` (`self.PS_TorchFire`) false false)
  (set `self.DefaultLightIntensity` (`LightComponentBase.Intensity` (`self.PointLight`))))

(event `self.OnEquipped`
  ;[1 1 1] On Equip/Unequip
  (`parent.OnEquipped`)
  (`self.ToggleVisualEffects` true))

(event `self.OnUnequipped`
  ;[1 1 1] On Equip/Unequip
  (`parent.OnUnequipped`)
  (`self.ToggleVisualEffects` false))

(event `ToggleVisualEffects`
  (params (On :type Boolean))
  ;[1 1 1] Toggle Visual Effects
  (`SceneComponent.SetVisibility` (`self.PointLight`) On false)
  (`ActorComponent.SetActive` (`self.PS_TorchFire`) On false))

(event `/Game/Blueprints/Equippable/PerformAction.PerformAction_1`
  ;[1 1 1] Perform Action 1 (Swing Torch)
  (`parent.PerformAction_1`)
  (if (and (`self.HasEnoughLight`) (`self.CanAttack`))
    (`|PlayMontage` (`Character.Mesh` (`self.Player`)) (`self.PrimaryActionAnimation`)
      (:`then`
        (`KismetSystemLibrary.K2_ClearAndInvalidateTimerHandle` (`self.LightRecoverTimer`))
        (`PrimitiveComponent.SetCollisionEnabled` (`self.FearCollider`) "QueryOnly")
        (set `self.CanAttack` false))
      (:`OnCompleted`
        (`PrimitiveComponent.SetCollisionEnabled` (`self.FearCollider`) "NoCollision" :!label _label)
        (set `self.LightLevel` (- (`self.LightLevel`) (`self.LightLevelLoss`)))
        (`self.SetLightLevel`)
        (`self.StartLightRecoveryTimer`)
        (set `self.CanAttack` true))
      (:`OnInterrupted`
        (goto _label)))))

(event `SetLightLevel`
  (bind _returnvalue (/ (`self.LightLevel`) (`self.MaxLightLevel`)))
  ;[1 1 1] Update Light Level Effects
  (`LightComponent.SetIntensity` (`self.PointLight`) (* (`self.DefaultLightIntensity`) _returnvalue))
  (`NiagaraComponent.SetVariableFloat` (`self.PS_TorchFire`) "User.SpawnRate" (* _returnvalue (`self.DefaultParticleSpawnrate`))))

(event `StartLightRecoveryTimer`
  ;[1 1 1] Light Level Recovery Timer
  (bind _returnvalue (`KismetSystemLibrary.K2_SetTimerDelegate` (delegate `RecoverLightLevel`) (`self.LightLevelRecoveryTime`) true))
  (set `self.LightRecoverTimer` _returnvalue))

(event `RecoverLightLevel`
  ;[1 1 1] Light Level Recovery Timer
  (set `self.LightLevel` (+ (`self.LightLevel`) 1.0))
  (`self.SetLightLevel`)
  (if (>= (`self.LightLevel`) (`self.MaxLightLevel`))
    (set `self.LightLevel` (`self.MaxLightLevel`))
    (`KismetSystemLibrary.K2_ClearAndInvalidateTimerHandle` (`self.LightRecoverTimer`))))

(fn `HasEnoughLight`
  (returns (CanAttack :type Boolean))
  (return (> (- (`self.LightLevel`) (`self.LightLevelLoss`)) 0.0)))

(fn `UserConstructionScript`
  (`parent.UserConstructionScript`))