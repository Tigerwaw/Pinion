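; Equippable musket that the player can aim, fire and reload through the parent equippable's three action events.
; Firing line-traces from the barrel, flashes the muzzle, then applies random-range damage through the Health interface or spawns sparks on other hits.
; Aiming changes walk speed and plays or reverses a camera boom timeline, switching rotation mode when it finishes.
; Reloading requires standing still and refills ammo when the player's timed progress bar completes.
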(event `StartAim`
  (bind _player (`self.Player`))
  (bind _camera_boom (`self.Camera Boom`))
  (bind _isdoingsecondaryaction (`/Game/CustomCharacter/PlayerCharacter/BP_ThirdPersonCharacter.IsDoingSecondaryAction` (`self.Player`)))
  ;[1 1 1] Toggle Aim
  (set `CharacterMovementComponent.MaxWalkSpeed` (`self.AimingWalkSpeed`) (`self.Character Movement`))
  (bind (_direction _boomarmlength _boomsocketoffset) (`Timeline|CameraZoomIn` :`NewTime` 0.2 :!via `PlayFromStart` :!label _label)
    (:`Update`
      (set `SpringArmComponent.TargetArmLength` _boomarmlength _camera_boom)
      (set `SpringArmComponent.SocketOffset` _boomsocketoffset _camera_boom))
    (:`Finished`
      (set `Pawn.bUseControllerRotationYaw` _isdoingsecondaryaction _player)
      (set `CharacterMovementComponent.bOrientRotationToMovement` (not _isdoingsecondaryaction) (`Character.CharacterMovement` _player)))))

(event `/Game/Blueprints/Items/Use.Use`
  (params (Player :type "/Game/CustomCharacter/PlayerCharacter/BP_ThirdPersonCharacter Object Reference"))
  (bind _player (`self.Player`))
  ;[1 1 1] Initialize Variables
  (`parent.Use` Player)
  (set `self.Character Movement` (`Character.CharacterMovement` _player))
  (set `self.Camera Boom` (`/Game/CustomCharacter/PlayerCharacter/BP_ThirdPersonCharacter.CameraBoom` _player))
  (set `self.Follow Camera` (`/Game/CustomCharacter/PlayerCharacter/BP_ThirdPersonCharacter.FollowCamera` _player))
  (set `self.Use Controller Rotation Yaw` (`Pawn.bUseControllerRotationYaw` _player)))

(event `CreateMuzzleFlash`
  (bind _barrel (`self.Barrel`))
  ;[1 1 1] Muzzle flash effect
  (`NiagaraFunctionLibrary.SpawnSystemAtLocation` (`self.ShootingParticlesystem`) (`SceneComponent.K2_GetComponentLocation` _barrel) (`KismetMathLibrary.Conv_VectorToRotator` (`SceneComponent.GetForwardVector` _barrel)))
  (`SceneComponent.SetVisibility` (`self.MuzzleFlashLight`) true false)
  (`KismetSystemLibrary.Delay` 0.05)
  (`SceneComponent.SetVisibility` (`self.MuzzleFlashLight`) false false))

(event `StopAim`
  ;[1 1 1] Toggle Aim
  (set `CharacterMovementComponent.MaxWalkSpeed` (`self.RegularWalkSpeed`) (`self.Character Movement`))
  (goto _label :!via `ReverseFromEnd`))

(event `/Game/Blueprints/Equippable/PerformAction.PerformAction_1`
  ;[1 1 1] Perform Action 1
  (`parent.PerformAction_1`)
  (`self.Shoot`))

(event `/Game/Blueprints/Equippable/PerformAction.PerformAction_2`
  ;[1 1 1] Perform Action 2
  (`parent.PerformAction_2`)
  (if (`/Game/CustomCharacter/PlayerCharacter/BP_ThirdPersonCharacter.IsDoingSecondaryAction` (`self.Player`))
    (`self.StartAim`)
    (else
      (`self.StopAim`))))

(event `Shoot`
  (bind _barrel (`self.Barrel`))
  (bind _returnvalue (`SceneComponent.K2_GetComponentLocation` _barrel))
  ;[1 1 1] Shoot
  (if (> (`self.CurrentLoadedAmount`) 0)
    (bind _outhit (`KismetSystemLibrary.LineTraceSingle` _returnvalue (+ _returnvalue (* (`SceneComponent.GetForwardVector` _barrel) (`self.ShootTraceRange`))) "TraceTypeQuery2" false (`|MakeArray` (`self.Player`) :!type "Actor Object Reference") "ForDuration"))
    (`self.CreateMuzzleFlash`)
    (`self.CheckHit` _outhit)
    (set `self.CurrentLoadedAmount` (- (`self.CurrentLoadedAmount`) 1))
    (`self.ShootEvent`)
    (else
      (`KismetSystemLibrary.PrintString` "Weapon is unloaded"))))

(event `/Game/Blueprints/Equippable/PerformAction.PerformAction_3`
  (bind _actionprogressbar (`/Game/CustomCharacter/PlayerCharacter/BP_ThirdPersonCharacter.ActionProgressbar` (`self.Player`)))
  ;[1 1 1] Perform Action 3
  (if (`self.CanReload`)
    (add `/Game/Blueprints/UI/CircleProgressbar.OnGenericActionFinished` _actionprogressbar (delegate `OnAction3Finished`))
    (`/Game/Blueprints/UI/CircleProgressbar.StartProgressTimer` _actionprogressbar (`self.ReloadTime`))))

(event `OnAction3Finished`
  ;[1 1 1] Perform Action 3
  (set `self.CurrentLoadedAmount` (`self.MaxLoadedAmount`))
  (`self.ReloadEvent`))

(event `CheckHit`
  (params (Hit :type "HitResult Structure"))
  (bind _damagerange (`self.DamageRange`))
  ;[1 1 1] On Hit
  (if (`KismetSystemLibrary.DoesImplementInterface` Hit_HitActor "/Game/Blueprints/CharacterStats/Health.Health_C")
    (message `/Game/Blueprints/CharacterStats/Health.Take Damage` Hit_HitActor (`KismetMathLibrary.RandomFloatInRange` (`.Value` (break `FloatRangeBound` (break `FloatRange` _damagerange))) (`.Value` (break `FloatRangeBound` (`.UpperBound` (break `FloatRange` _damagerange))))) Hit_ImpactPoint (`self.Player`))
    (else
      (`NiagaraFunctionLibrary.SpawnSystemAtLocation` "/Game/Particles/PS_SparkBurst.PS_SparkBurst" Hit_ImpactPoint))))

(fn `CanReload`
  (returns (CanReload :type Boolean))
  (return (and (< (`self.CurrentLoadedAmount`) (`self.MaxLoadedAmount`)) (not (`/Game/CustomCharacter/PlayerCharacter/BP_ThirdPersonCharacter.IsCharacterMoving` (`self.Player`))))))

(fn `UserConstructionScript`
  (`parent.UserConstructionScript`))