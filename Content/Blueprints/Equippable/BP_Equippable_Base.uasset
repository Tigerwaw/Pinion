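; Base equippable item that the player can pick up, equip, stow, drop and use for actions.
; Interacting calls the player's EquipAndUnequip, while Equip and Unequip snap the item between two mesh sockets and fire empty hooks.
; Dropping unequips if the held class matches, then detaches, moves it and enables custom depth.
; The primary action pulses a player flag for one tick, the secondary toggles one, and the third is empty.
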(event `/Game/Blueprints/Interactables/Interact.Interact`
  (params (Player :type "/Game/CustomCharacter/PlayerCharacter/BP_ThirdPersonCharacter Object Reference"))
  (`parent.Interact` Player)
  (set `self.PickedUp` true)
  (`/Game/Blueprints/Items/Use.Use` Player))

(event `/Game/Blueprints/Items/Use.Use`
  (params (Player :type "/Game/CustomCharacter/PlayerCharacter/BP_ThirdPersonCharacter Object Reference"))
  ;[1 1 1] Equip Item
  (bind _output_get (set `self.Player` Player))
  (`/Game/CustomCharacter/PlayerCharacter/BP_ThirdPersonCharacter.EquipAndUnequip` _output_get self))

(event `self.DropItem`
  (params (DropLocation :type "Vector Structure"))
  (bind (_iteminfo_icon _iteminfo_name _iteminfo_description _iteminfo_itemclass) (break `/Game/Blueprints/Items/ItemInfoStructure` (`self.ItemInfo`)))
  ;[1 1 1] Drop Item
  (if (== (`GameplayStatics.GetObjectClass` (`/Game/CustomCharacter/PlayerCharacter/BP_ThirdPersonCharacter.Equipped` (`self.Player`))) _iteminfo_itemclass)
    (`/Game/CustomCharacter/PlayerCharacter/BP_ThirdPersonCharacter.EquipAndUnequip` (`self.Player`) self))
  (`self.K2_DetachFromActor` self "KeepRelative" "KeepRelative" "KeepRelative")
  (`SceneComponent.K2_SetWorldLocation` (`self.DefaultSceneRoot`) DropLocation false false)
  (`PrimitiveComponent.SetRenderCustomDepth` (`self.ItemMesh`) true)
  (set `self.PickedUp` false))

(event `/Game/Blueprints/Equippable/PerformAction.PerformAction_1`
  (params (Player :type "/Game/CustomCharacter/PlayerCharacter/BP_ThirdPersonCharacter Object Reference"))
  ;[1 1 1] Perform Action 1
  (set `/Game/CustomCharacter/PlayerCharacter/BP_ThirdPersonCharacter.IsDoingPrimaryAction` true Player)
  (`KismetSystemLibrary.DelayUntilNextTick`)
  (set `/Game/CustomCharacter/PlayerCharacter/BP_ThirdPersonCharacter.IsDoingPrimaryAction` false Player))

(event `OnEquipped`)

(event `/Game/Blueprints/Equippable/PerformAction.PerformAction_2`
  (params (Player :type "/Game/CustomCharacter/PlayerCharacter/BP_ThirdPersonCharacter Object Reference"))
  ;[1 1 1] Perform Action 2
  (set `/Game/CustomCharacter/PlayerCharacter/BP_ThirdPersonCharacter.IsDoingSecondaryAction` (not (`/Game/CustomCharacter/PlayerCharacter/BP_ThirdPersonCharacter.IsDoingSecondaryAction` Player)) Player))

(event `OnUnequipped`)

(event `/Game/Blueprints/Equippable/PerformAction.PerformAction_3`
  (params (Player :type "/Game/CustomCharacter/PlayerCharacter/BP_ThirdPersonCharacter Object Reference")))

(fn `Equip`
  (`SceneComponent.K2_AttachToComponent` (`self.DefaultSceneRoot`) (`Character.Mesh` (`self.Player`)) (`self.EquippedSocketName`) "SnapToTarget" "SnapToTarget" "SnapToTarget" true)
  (`self.OnEquipped`))

(fn `Unequip`
  (`SceneComponent.K2_AttachToComponent` (`self.DefaultSceneRoot`) (`Character.Mesh` (`self.Player`)) (`self.UnequippedSocketName`) "SnapToTarget" "SnapToTarget" "SnapToTarget" true)
  (`self.OnUnequipped`))

(fn `UserConstructionScript`
  (`parent.UserConstructionScript`))