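; Base character Blueprint that handles health, damage, healing and death.
; TakeDamage and Heal adjust CurrentHealth, then call CheckHealthStatus, which caps it at MaxHealth or clamps it to zero and triggers Death.
; TakeDamage also spawns a particle system at the hit location.
; Death sets the IsDead flag and destroys the actor after a short delay.
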(event `CheckHealthStatus`
  (if (> (`self.CurrentHealth`) (`self.MaxHealth`))
    (set `self.CurrentHealth` (`self.MaxHealth`))
    (elif (<= (`self.CurrentHealth`) 0.0)
      (set `self.CurrentHealth` 0.0)
      (`self.Death`))))

(event `self.Take Damage`
  (params (DamageAmount :type "Float (double-precision)") (HitLocation :type "Vector Structure") (DamagedBy :type "Actor Object Reference"))
  (set `self.CurrentHealth` (- (`self.CurrentHealth`) DamageAmount))
  (`self.CheckHealthStatus`)
  (`NiagaraFunctionLibrary.SpawnSystemAtLocation` (`self.TakeDamageParticle`) HitLocation))

(event `self.Heal`
  (params (HealAmount :type "Float (double-precision)"))
  (set `self.CurrentHealth` (+ (`self.CurrentHealth`) HealAmount))
  (`self.CheckHealthStatus`))

(event `self.Death`
  (set `self.IsDead` true)
  (`KismetSystemLibrary.Delay` 5.0)
  (`self.K2_DestroyActor`))

(fn `UserConstructionScript`)